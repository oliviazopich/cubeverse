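; BP_Item is a pickup item actor for the inventory system, with its data held in the BPCItemData component.
; BeginPlay copies CanPickup into that component; ToggleCanPickup only ever sets both to true.
; FocusTarget looks up the item's data table row to build a "Pickup {Item}" prompt.
; On Destroyed, it adds itself uniquely to ActorsRemoved in the first-person game mode's level save data.
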(event Custom|Toggle%20Can%20Pickup
  (Variables|Default|SetCanPickup? true)
  (Variables|/Game/Inventory_System/BPC_ItemData.BPC_ItemData_C|SetCanPickup? (Variables|Default|GetBPC_ItemData) true))

(event EventBeginPlay
  (Variables|/Game/Inventory_System/BPC_ItemData.BPC_ItemData_C|SetCanPickup? (Variables|Default|GetBPC_ItemData) (Variables|Default|GetCanPickup?))
  (Variables|Default|SetItemDataRef (Variables|Default|GetBPC_ItemData)))

(event Collision|EventActorBeginOverlap
  (params (OtherActor :type Actor%20Object%20Reference)))

(event EventTick
  (params (DeltaSeconds :type Float%20%28single-precision%29)))

(event EventDestroyed
  (bind _asbp_first_person_game_mode (Utilities|Casting|CastToBP_FirstPersonGameMode (Game|GetGameMode)))
  (Utilities|Array|AddUnique (Variables|/Game/SaveSystem/BP_SaveData_Level.BP_SaveData_Level_C|GetActorsRemoved (Variables|/Game/FirstPerson/Blueprints/BP_FirstPersonGameMode.BP_FirstPersonGameMode_C|GetSaveDataLevel _asbp_first_person_game_mode)) (Utilities|ResolveSoftReference self)))

(fn ConstructionScript)

(fn FocusTarget
  (bind _bpc_itemdata (Variables|Default|GetBPC_ItemData))
  (bind _itemid (Variables|/Game/Inventory_System/BPC_ItemData.BPC_ItemData_C|GetItemID _bpc_itemdata))
  (bind (_datatable _rowname) (Utilities|Struct|BreakDataTableRowHandle _itemid))
  (bind _returnvalue (Utilities|GetDataTableRow _datatable _rowname)
    (:then
      (return (Utilities|Text|FormatText "Pickup {Item} " (.Name (Utilities|Struct|BreakS_ItemData _returnvalue)))))))