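; BP_Apple is a usable healing item in the inventory system.
; Its Use event gets the player character's BP_MyController and, if current health is below maximum, calls HealPlayer with HealAmount and destroys the apple.
; At full health the apple is kept and a "Health is full" message is printed.
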(event EventBeginPlay
  (|CallParentFunction) ; This node is disabled and will not be called.\nDrag off pins to build functionality.
)

(event Collision|EventActorBeginOverlap
  (params (OtherActor :type Actor%20Object%20Reference))
  (|CallParentFunction OtherActor) ; This node is disabled and will not be called.\nDrag off pins to build functionality.
)

(event EventTick
  (params (DeltaSeconds :type Float%20%28single-precision%29))
  (|CallParentFunction DeltaSeconds))

(event EventUse
  (bind _asbp_first_person_character (Utilities|Casting|CastToBP_FirstPersonCharacter (Game|GetPlayerCharacter 0)))
  (bind _asbp_my_controller (Utilities|Casting|CastToBP_MyController (Pawn|GetController _asbp_first_person_character)))
  (if (< (Variables|/Game/FirstPerson/Blueprints/BP_MyController.BP_MyController_C|GetCurrentHealth _asbp_my_controller) (Variables|/Game/FirstPerson/Blueprints/BP_MyController.BP_MyController_C|GetMaxHealth _asbp_my_controller))
    (Default|HealPlayer _asbp_my_controller (Variables|Default|GetHeal%20Amount))
    (Actor|DestroyActor)
    (else
      (Development|PrintString "Health is full"))))

(fn ConstructionScript
  (|CallParentFunction))