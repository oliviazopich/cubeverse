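; BP_Cobble is an inventory item, apparently cobblestone, that places blocks in the world.
; On Use, it line traces 600 units from the first-person camera, snaps the impact point to a TileSize grid and spawns a Block there without checking for a hit.
; It then re-enables its cube's collision, which a separate event turns off.
; Another event marks the item as pickable, while OnInteract is empty and overlap defers to the parent.
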(event Custom|CustomEvent_1
  (Variables|Default|SetCanPickup? true)
  (Variables|/Game/Inventory_System/BPC_ItemData.BPC_ItemData_C|SetCanPickup? (Variables|Default|GetBPC_ItemData) true))

(event EventUse
  (bind _tilesize (Variables|Default|GetTileSize))
  (bind _asbp_first_person_character (Utilities|Casting|CastToBP_FirstPersonCharacter (Game|GetPlayerCharacter 0)))
  (bind _outhit (Collision|LineTraceByChannel (Transformation|GetWorldLocation (Variables|/Game/FirstPerson/Blueprints/BP_FirstPersonCharacter.BP_FirstPersonCharacter_C|GetFirstPersonCamera _asbp_first_person_character)) (+ (Transformation|GetWorldLocation (Variables|/Game/FirstPerson/Blueprints/BP_FirstPersonCharacter.BP_FirstPersonCharacter_C|GetFirstPersonCamera _asbp_first_person_character)) (* (Math|Vector|GetForwardVector (Variables|/Game/FirstPerson/Blueprints/BP_FirstPersonCharacter.BP_FirstPersonCharacter_C|GetFirstPersonCamera _asbp_first_person_character)) 6e+02)) "TraceTypeQuery1" false 0 "None" false))
  (Game|SpawnActorfromClass (Variables|Default|GetBlock) (Math|Transform|MakeTransform (Math|Vector|MakeVector (Math|Float|SnapToGrid(Float) (.X (Math|Vector|BreakVector (.ImpactPoint (Collision|BreakHitResult _outhit)))) _tilesize) (Math|Float|SnapToGrid(Float) (.Y (Math|Vector|BreakVector (.ImpactPoint (Collision|BreakHitResult _outhit)))) _tilesize) (Math|Float|SnapToGrid(Float) (.Z (Math|Vector|BreakVector (.ImpactPoint (Collision|BreakHitResult _outhit)))) _tilesize))) "Undefined" "MultiplyWithRoot" 0 0)
  (Collision|SetCollisionEnabled (Variables|Default|GetCube) "QueryAndPhysics"))

(event Collision|EventActorBeginOverlap
  (params (OtherActor :type Actor%20Object%20Reference))
  (|CallParentFunction OtherActor))

(event EventTick
  (params (DeltaSeconds :type Float%20%28single-precision%29))
  (|CallParentFunction DeltaSeconds) ; This node is disabled and will not be called.\nDrag off pins to build functionality.
)

(event EventOnInteract)

(event EventBeginPlay
  (|CallParentFunction))

(event EventTurnOffCollisions
  (Collision|SetCollisionEnabled (Variables|Default|GetCube) "NoCollision"))

(fn ConstructionScript
  (|CallParentFunction))