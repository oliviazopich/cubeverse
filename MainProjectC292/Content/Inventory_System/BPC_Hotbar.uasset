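; Hotbar component, built on a parent inventory component, that handles item slot selection and restores hotbar contents from saved player data.
; On BeginPlay it loads hotbar data from the game instance if a save exists, otherwise it just refreshes the inventory.
; Number keys and scroll input actions set a wrapping index across nine slots, highlight that slot on the HUD hotbar and refresh the inventory.
; A getter exposes the slots.
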(event Input|EnhancedActionEvents|EnhancedInputActionIA_HotbarUp
  (params (ActionValue :type Boolean) (ElapsedSeconds :type Float%20%28double-precision%29) (TriggeredSeconds :type Float%20%28double-precision%29) (InputAction :type Input%20Action%20Object%20Reference :default "/Game/FirstPerson/Input/Actions/IA_HotbarUp.IA_HotbarUp"))
  (bind _output_get (Variables|Default|SetScrollIndex (Math|Integer|Clamp(Integer) (+ (Variables|Default|GetScrollIndex) 1) -1 9)))
  (if (== _output_get 9)
    (Variables|Default|SetScrollIndex 0))
  (CallFunction|GetSelectedSlot (Variables|Default|GetScrollIndex)))

(event Input|EnhancedActionEvents|EnhancedInputActionIA_HotbarDown
  (params (ActionValue :type Boolean) (ElapsedSeconds :type Float%20%28double-precision%29) (TriggeredSeconds :type Float%20%28double-precision%29) (InputAction :type Input%20Action%20Object%20Reference :default "/Game/FirstPerson/Input/Actions/IA_HotbarDown.IA_HotbarDown"))
  (bind _output_get (Variables|Default|SetScrollIndex (Math|Integer|Clamp(Integer) (- (Variables|Default|GetScrollIndex) 1) -1 9)))
  (if (== _output_get -1)
    (Variables|Default|SetScrollIndex 8))
  (CallFunction|GetSelectedSlot (Variables|Default|GetScrollIndex)))

(event EventBeginPlay
  (|CallParentFunction)
  (bind _returnvalue (SaveGame|DoesSaveGameExist "slot1"))
  (if _returnvalue
    (bind _savedata (Class|BPISaveSystem|GetSaveData(Message) (Game|GetGameInstance)))
    (Utilities|IsValid (.PlayerData (Utilities|Struct|BreakS_SaveData _savedata))
      (:Is%20Valid
        (SaveSystem|LoadHotbarData (Variables|/Game/SaveSystem/BP_SaveData_Player.BP_SaveData_Player_C|GetHotbarData (.PlayerData (Utilities|Struct|BreakS_SaveData _savedata))))))
    (else
      (CallFunction|UpdateInventory))))

(event EventTick
  (params (DeltaSeconds :type Float%20%28single-precision%29)))

(event Input|KeyboardEvents|9
  (params (Key :type Key%20Structure :default "None"))
  (:Pressed
    (bind _output_get (Variables|Default|SetScrollIndex 8))
    (CallFunction|GetSelectedSlot _output_get)))

(event Input|KeyboardEvents|1
  (params (Key :type Key%20Structure :default "None"))
  (:Pressed
    (bind _output_get (Variables|Default|SetScrollIndex 0))
    (CallFunction|GetSelectedSlot _output_get)))

(event Input|KeyboardEvents|2
  (params (Key :type Key%20Structure :default "None"))
  (:Pressed
    (bind _output_get (Variables|Default|SetScrollIndex 1))
    (CallFunction|GetSelectedSlot _output_get)))

(event Input|KeyboardEvents|3
  (params (Key :type Key%20Structure :default "None"))
  (:Pressed
    (bind _output_get (Variables|Default|SetScrollIndex 2))
    (CallFunction|GetSelectedSlot _output_get)))

(event Input|KeyboardEvents|4
  (params (Key :type Key%20Structure :default "None"))
  (:Pressed
    (bind _output_get (Variables|Default|SetScrollIndex 3))
    (CallFunction|GetSelectedSlot _output_get)))

(event Input|KeyboardEvents|5
  (params (Key :type Key%20Structure :default "None"))
  (:Pressed
    (bind _output_get (Variables|Default|SetScrollIndex 4))
    (CallFunction|GetSelectedSlot _output_get)))

(event Input|KeyboardEvents|6
  (params (Key :type Key%20Structure :default "None"))
  (:Pressed
    (bind _output_get (Variables|Default|SetScrollIndex 5))
    (CallFunction|GetSelectedSlot _output_get)))

(event Input|KeyboardEvents|7
  (params (Key :type Key%20Structure :default "None"))
  (:Pressed
    (bind _output_get (Variables|Default|SetScrollIndex 6))
    (CallFunction|GetSelectedSlot _output_get)))

(event Input|KeyboardEvents|8
  (params (Key :type Key%20Structure :default "None"))
  (:Pressed
    (bind _output_get (Variables|Default|SetScrollIndex 7))
    (CallFunction|GetSelectedSlot _output_get)))

(fn GetSelectedSlot
  (params (Index :type Integer))
  (bind _itemslots (Variables|Default|GetItemSlots))
  (bind _output (Utilities|Array|Get(acopy) _itemslots Index))
  (LocalVariables|SetLocal_ItemID (.itemid _output))
  (LocalVariables|SetLocal_ItemQuantity (.itemquantity _output))
  (Default|SelectedSlot (Variables|/Game/FirstPerson/UI/WB_PlayerHUD.WB_PlayerHUD_C|GetWB_HotbarDisplay (CallFunction|GetPlayerHUD)) Index)
  (CallFunction|UpdateInventory)
  (return Index))

(fn GetHotbarData
  (return (Variables|Default|GetItemSlots)))

(fn LoadHotbarData
  (params (HotbarData :type Array%20of%20S%20Item%20Slot%20Structures))
  (Variables|Default|SetItemSlots HotbarData)
  (Utilities|Array|Resize (Variables|Default|GetItemSlots) (Variables|Default|GetInventorySize))
  (CallFunction|UpdateInventory))