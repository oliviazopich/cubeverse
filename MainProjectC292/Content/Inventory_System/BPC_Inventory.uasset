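; Player inventory component that stores item stacks in slots and detects nearby interactables.
; Once started, a looping timer sphere-traces around the owner to update the target and prompt widget; IA_Interact forwards to the target's BPC_ItemData.
; Pickup tops up matching stacks or fills empty slots, one unit per call, using DT_ItemData stack limits.
; Stacks can be halved or used, spawning the item's Effect actor within a forward cone, then broadcasting inventory updates.
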(event Custom|CreateInteractMessage
  (bind _returnvalue (UserInterface|CreateWidget "/Game/Inventory_System/UI/WB_InteractMessage.WB_InteractMessage_C"))
  (bind _output_get (Variables|Default|SetWB_InteractMessage _returnvalue))
  (UserInterface|Viewport|AddtoViewport _output_get 0))

(event Custom|BeginInteraction
  (Utilities|Time|SetTimerbyEvent (delegate Custom|UpdateInteraction) 0.2 true))

(event Custom|UpdateInteraction
  (CallFunction|Interaction))

(event Custom|UpdateInventory
  (Default|CallOnInventoryUpdated))

(event Input|EnhancedActionEvents|EnhancedInputActionIA_Interact
  (params (ActionValue :type Boolean) (ElapsedSeconds :type Float%20%28double-precision%29) (TriggeredSeconds :type Float%20%28double-precision%29) (InputAction :type Input%20Action%20Object%20Reference :default "/Game/FirstPerson/Input/Actions/IA_Interact.IA_Interact"))
  (:Started
    (bind _targetactor (Variables|Default|GetTargetActor)
      (:then
        (Utilities|IsValid (Actor|GetComponentbyClass _targetactor "/Game/Inventory_System/BPC_ItemData.BPC_ItemData_C")
          (:Is%20Valid
            (Class|BPIInteract|Interact(Message) (Actor|GetComponentbyClass _targetactor "/Game/Inventory_System/BPC_ItemData.BPC_ItemData_C") (.AsBP%20First%20Person%20Character (Utilities|Casting|CastToBP_FirstPersonCharacter (Game|GetPlayerCharacter 0)))))))
      (:else))))

(event EventBeginPlay
  (Utilities|Array|Resize (Variables|Default|GetItemSlots) (Variables|Default|GetInventorySize)))

(fn PrintInventory
  (for (_array_element _array_index) (Variables|Default|GetItemSlots)
    (Development|PrintString (Utilities|String|Append (Utilities|String|ToString(Integer) _array_index) ": " (Utilities|String|ToString(Name) (.ItemID (Utilities|Struct|BreakS_ItemSlot _array_element))) " = " (Utilities|String|ToString(Integer) (.ItemQuantity (Utilities|Struct|BreakS_ItemSlot _array_element)))))))

(fn Interaction
  (bind _returnvalue (Components|GetOwner))
  (bind _returnvalue_2 (Transformation|GetActorLocation _returnvalue))
  (bind (_outhit _returnvalue_3) (Collision|SphereTraceByChannel _returnvalue_2 _returnvalue_2 (Variables|Default|GetInteractRadius) "TraceTypeQuery3" false (Utilities|Array|MakeArray (Components|GetOwner)) "None"))
  (if _returnvalue_3
    (if (!= (.HitActor (Collision|BreakHitResult _outhit)) (Variables|Default|GetTargetActor))
      (bind _output_get (Variables|Default|SetTargetActor (.HitActor (Collision|BreakHitResult _outhit))))
      (bind _message (Class|BPIInteract|FocusTarget(Message) _output_get))
      (Default|SetInteractMessage (Variables|Default|GetWB_InteractMessage) _message))
    (else
      (Variables|Default|SetTargetActor 0)
      (Default|SetInteractMessage (Variables|Default|GetWB_InteractMessage)))))

(fn Pickup
  (params (ItemID :type Name) (ItemQuantity :type Integer))
  (bind (_success _index) (CallFunction|AnySlotAvailable))
  (bind _output_get (LocalVariables|SetLocal%20Item%20Quantity ItemQuantity))
  (while (and (> _output_get 0) (not (LocalVariables|GetLocal_%20IsFull)))
    (bind (_success_2 _index_2) (CallFunction|FindSlot ItemID))
    (if _success_2
      (CallFunction|AddtoStack _index_2 1)
      (Math|Integer|DecrementInt (LocalVariables|GetLocal%20Item%20Quantity)
        (:%20%20
          (return true 0)))
      (elif _success
        (CallFunction|CreateNewStack ItemID 1 _index)
        (Math|Integer|DecrementInt (LocalVariables|GetLocal%20Item%20Quantity)
          (:%20%20
            (return true 0)))
        (else
          (LocalVariables|SetLocal_%20IsFull true)))))
  (return (not (LocalVariables|GetLocal_%20IsFull)) (LocalVariables|GetLocal%20Item%20Quantity)))

(fn FindSlot
  (params (ItemID :type Name))
  (for (_array_element _array_index) (Variables|Default|GetItemSlots)
    (if (and (== ItemID (.ItemID (Utilities|Struct|BreakS_ItemSlot _array_element))) (< (.ItemQuantity (Utilities|Struct|BreakS_ItemSlot _array_element)) (CallFunction|GetMaxStackSize ItemID)))
      (return true _array_index)))
  (return false -1))

(fn GetMaxStackSize
  (params (ItemID :type Name))
  (bind _returnvalue (Utilities|GetDataTableRow "/Game/Inventory_System/ItemData/DT_ItemData.DT_ItemData" ItemID)
    (:then
      (return (.SlotQuantity (Utilities|Struct|BreakS_ItemData _returnvalue))))))

(fn AddtoStack
  (params (Index :type Integer) (ItemQuantity :type Integer))
  (bind _itemslots (Variables|Default|GetItemSlots))
  (bind _output (Utilities|Array|Get(acopy) _itemslots Index))
  (Utilities|Array|SetArrayElem (Variables|Default|GetItemSlots) Index (Utilities|Struct|MakeS_ItemSlot (.itemid _output) (+ (.itemquantity _output) ItemQuantity))))

(fn AnySlotAvailable
  (for (_array_element _array_index) (Variables|Default|GetItemSlots)
    (if (== (.ItemQuantity (Utilities|Struct|BreakS_ItemSlot _array_element)) 0)
      (return true _array_index)))
  (return false -1))

(fn CreateNewStack
  (params (ItemID :type Name) (ItemQuantity :type Integer) (Index :type Integer))
  (Utilities|Array|SetArrayElem (Variables|Default|GetItemSlots) Index (Utilities|Struct|MakeS_ItemSlot ItemID ItemQuantity)))

(fn SplitStack
  (params (Index :type Integer))
  (bind (_success _index) (CallFunction|AnySlotAvailable))
  (bind _itemslots (Variables|Default|GetItemSlots))
  (bind _output (Utilities|Array|Get(acopy) _itemslots Index))
  (LocalVariables|SetLocal_ItemID (.itemid _output))
  (LocalVariables|SetLocal_ItemQuantity (.itemquantity _output))
  (Utilities|FlowControl|Sequence
    (:then_0
      (if (not (== (LocalVariables|GetLocal_ItemQuantity) 1))
        (if _success
          (LocalVariables|SetLocal_SplitQuantity (/ (LocalVariables|GetLocal_ItemQuantity) 2))
          (Utilities|Array|SetArrayElem (Variables|Default|GetItemSlots) _index (Utilities|Struct|MakeS_ItemSlot (LocalVariables|GetLocal_ItemID) (LocalVariables|GetLocal_SplitQuantity)))
          (Utilities|Array|SetArrayElem (Variables|Default|GetItemSlots) Index (Utilities|Struct|MakeS_ItemSlot (LocalVariables|GetLocal_ItemID) (- (LocalVariables|GetLocal_ItemQuantity) (LocalVariables|GetLocal_SplitQuantity)))))))
    (:then_1
      (bind _returnvalue (Utilities|GetDataTableRow "/Game/Inventory_System/ItemData/DT_ItemData.DT_ItemData" (LocalVariables|GetLocal_ItemID))
        (:then
          (CallFunction|UpdateInventory))))))

(fn UseItem
  (params (Index :type Integer))
  (bind _itemslots (Variables|Default|GetItemSlots))
  (bind _output (Utilities|Array|Get(acopy) _itemslots Index))
  (LocalVariables|SetLocal_ItemID (.itemid _output))
  (LocalVariables|SetLocal_ItemQuantity (.itemquantity _output))
  (Utilities|FlowControl|Sequence
    (:then_0
      (if (== (LocalVariables|GetLocal_ItemQuantity) 1)
        (Utilities|Array|SetArrayElem (Variables|Default|GetItemSlots) Index (Utilities|Struct|MakeS_ItemSlot "None" 0))
        (else
          (CallFunction|UpdateStack Index 1)))
      (Game|SpawnActorfromClass (Utilities|Struct|BreakS_ItemData (CallFunction|GetItemData (LocalVariables|GetLocal_ItemID))) (Math|Transform|MakeTransform (CallFunction|GetDropLocation) "0, 0, 0" "1.000000,1.000000,1.000000") "AlwaysSpawn" "MultiplyWithRoot" 0 0))
    (:then_1
      (bind _returnvalue (Utilities|GetDataTableRow "/Game/Inventory_System/ItemData/DT_ItemData.DT_ItemData" (LocalVariables|GetLocal_ItemID))
        (:then
          (CallFunction|UpdateInventory))))))

(fn UpdateStack
  (params (Index :type Integer) (ItemQuantity :type Integer))
  (bind _itemslots (Variables|Default|GetItemSlots))
  (bind _output (Utilities|Array|Get(acopy) _itemslots Index))
  (Utilities|Struct|SetmembersinS_ItemSlot _output (- (Utilities|Struct|BreakS_ItemSlot _output) ItemQuantity)))

(fn GetDropLocation
  (bind _returnvalue (Components|GetOwner))
  (return (+ (Transformation|GetActorLocation _returnvalue) (* (Math|Random|RandomUnitVectorinConeinDegrees (Transformation|GetActorForwardVector _returnvalue) 55.0) 1.2e+02))))

(fn GetItemData
  (params (ItemID :type Name))
  (bind _returnvalue (Utilities|GetDataTableRow "/Game/Inventory_System/ItemData/DT_ItemData.DT_ItemData" ItemID)
    (:then
      (return _returnvalue))))