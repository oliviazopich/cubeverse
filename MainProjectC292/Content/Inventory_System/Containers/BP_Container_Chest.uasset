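; BP_Container_Chest is an inventory system chest container that toggles between open and closed.
; OnInteract and UpdateContainer share the same logic, which flips IsOpen and plays the matching open or close sound from ContainerSFX at the chest's location.
; The graphs contain no lid animation or inventory logic, and the construction script only calls its parent.
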(event EventBeginPlay
  (|CallParentFunction) ; This node is disabled and will not be called.\nDrag off pins to build functionality.
)

(event EventOnInteract
  (bind _returnvalue (Transformation|GetActorLocation))
  (bind _container_sfx (Variables|Default|GetContainer%20SFX))
  (bind (_open _close) (Utilities|Struct|BreakS_ContainerSFX _container_sfx))
  (if (not (Variables|Default|GetIsOpen?))
    (Variables|Default|SetIsOpen? true)
    (Audio|PlaySoundatLocation _open _returnvalue "0, 0, 0" 1.0 1.0 0.0 0 0 0 0)
    (else
      (Variables|Default|SetIsOpen? false)
      (Audio|PlaySoundatLocation _close _returnvalue "0, 0, 0" 1.0 1.0 0.0 0 0 0 0))))

(event EventUpdateContainer
  (bind _returnvalue (Transformation|GetActorLocation))
  (bind _container_sfx (Variables|Default|GetContainer%20SFX))
  (bind (_open _close) (Utilities|Struct|BreakS_ContainerSFX _container_sfx))
  (if (not (Variables|Default|GetIsOpen?))
    (Variables|Default|SetIsOpen? true)
    (Audio|PlaySoundatLocation _open _returnvalue "0, 0, 0" 1.0 1.0 0.0 0 0 0 0)
    (else
      (Variables|Default|SetIsOpen? false)
      (Audio|PlaySoundatLocation _close _returnvalue "0, 0, 0" 1.0 1.0 0.0 0 0 0 0))))

(fn ConstructionScript
  (|CallParentFunction))