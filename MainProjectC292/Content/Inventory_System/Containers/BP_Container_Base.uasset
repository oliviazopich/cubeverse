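; Base actor for searchable world containers that hold an inventory component and show a "Search" prompt with the container's name.
; Shortly after BeginPlay, it restores slots from level save data, or uses default contents if no save exists, resized to container size.
; Interacting opens a container display on the player HUD.
; Saving appends the component and its slots to parallel game-mode arrays, and loading matches by component reference.
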(event Custom|Update%20Container)

(event EventBeginPlay
  (bind _bpc_inventory (Variables|Default|GetBPC_Inventory))
  (Utilities|FlowControl|Delay 0.2)
  (bind _asbp_first_person_game_mode (Utilities|Casting|CastToBP_FirstPersonGameMode (Game|GetGameMode)))
  (bind _returnvalue (SaveGame|DoesSaveGameExist (Variables|/Game/FirstPerson/Blueprints/BP_FirstPersonGameMode.BP_FirstPersonGameMode_C|GetLevelData _asbp_first_person_game_mode)))
  (if _returnvalue
    (bind _savedata (Class|BPISaveSystem|GetSaveData(Message) (Game|GetGameMode)))
    (Utilities|IsValid (.LevelData (Utilities|Struct|BreakS_SaveData _savedata))
      (:Is%20Valid
        (CallFunction|LoadContainerData (Variables|/Game/SaveSystem/BP_SaveData_Level.BP_SaveData_Level_C|GetContainerData (.LevelData (Utilities|Struct|BreakS_SaveData _savedata))))))
    (else
      (Variables|/Game/Inventory_System/BPC_Inventory.BPC_Inventory_C|SetItemSlots _bpc_inventory (Variables|Default|GetContainerContent))
      (Utilities|Array|Resize (Variables|/Game/Inventory_System/BPC_Inventory.BPC_Inventory_C|GetItemSlots _bpc_inventory) (Variables|Default|GetContainerSize)))))

(event EventInteract
  (params (BP_FirstPerson :type BP%20First%20Person%20Character%20Object%20Reference))
  (bind _asbp_my_controller (Utilities|Casting|CastToBP_MyController (Game|GetPlayerController 0)))
  (bind _returnvalue (Default|CreateContainerDisplay (Variables|/Game/FirstPerson/Blueprints/BP_MyController.BP_MyController_C|GetWB_PlayerHUD _asbp_my_controller) (Variables|Default|GetBPC_Inventory)))
  (EventDispatchers|BindEventtoOnContainerClosed _returnvalue (EventDispatchers|CreateEvent :!event Custom|Update%20Container)))

(fn ConstructionScript)

(fn GetContainerData
  (bind _asbp_first_person_game_mode (Utilities|Casting|CastToBP_FirstPersonGameMode (Game|GetGameMode)))
  (Utilities|Array|Add (.Containers (Utilities|Struct|BreakS_ContainerData (Variables|/Game/SaveSystem/BP_SaveData_Level.BP_SaveData_Level_C|GetContainerData (Variables|/Game/FirstPerson/Blueprints/BP_FirstPersonGameMode.BP_FirstPersonGameMode_C|GetSaveDataLevel _asbp_first_person_game_mode)))) (Utilities|ResolveSoftReference (Variables|Default|GetBPC_Inventory)))
  (Utilities|Array|Add (.ContainerInventories (Utilities|Struct|BreakS_ContainerData (Variables|/Game/SaveSystem/BP_SaveData_Level.BP_SaveData_Level_C|GetContainerData (Variables|/Game/FirstPerson/Blueprints/BP_FirstPersonGameMode.BP_FirstPersonGameMode_C|GetSaveDataLevel _asbp_first_person_game_mode)))) (Utilities|Struct|MakeS_ContainerInventory (Variables|/Game/Inventory_System/BPC_Inventory.BPC_Inventory_C|GetItemSlots (Variables|Default|GetBPC_Inventory))))
  (return (Variables|/Game/SaveSystem/BP_SaveData_Level.BP_SaveData_Level_C|GetContainerData (Variables|/Game/FirstPerson/Blueprints/BP_FirstPersonGameMode.BP_FirstPersonGameMode_C|GetSaveDataLevel _asbp_first_person_game_mode))))

(fn LoadContainerData
  (params (ContainerData :type S%20Container%20Data%20Structure))
  (bind (_containers _containerinventories) (Utilities|Struct|BreakS_ContainerData ContainerData))
  (bind _output_get (Variables|/Game/Inventory_System/BPC_Inventory.BPC_Inventory_C|SetItemSlots (Variables|Default|GetBPC_Inventory) (Utilities|Struct|BreakS_ContainerInventory (Utilities|Array|Get(acopy) _containerinventories (Utilities|Array|FindItem _containers (Utilities|ResolveSoftReference (Variables|Default|GetBPC_Inventory)))))))
  (Utilities|Array|Resize _output_get (Variables|Default|GetContainerSize)))

(fn FocusTarget
  (return (Utilities|Text|FormatText "Search {Container}" (Variables|Default|GetContainerName))))

(fn GetActorSoundParams
  (return 0))