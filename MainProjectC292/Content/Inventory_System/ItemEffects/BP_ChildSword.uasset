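; BP_ChildSword is an inventory item effect that puts a sword in the first-person player's hand.
; On BeginPlay it casts the player pawn to BP_FirstPersonCharacter and caches it as Character.
; It then spawns a BP_Item_Sword at a placeholder point high above the origin and snaps its root to the hand socket on the first-person mesh.
; The construction script only calls its parent, and no other logic runs.
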(event EventBeginPlay
  (bind _asbp_first_person_character (Utilities|Casting|CastToBP_FirstPersonCharacter (Game|Player|GetPlayerPawn 0)))
  (Variables|Default|SetCharacter _asbp_first_person_character)
  (bind _returnvalue (Game|SpawnActorfromClass "/Game/Inventory_System/Items/BP_Item_Sword.BP_Item_Sword_C" (Math|Transform|MakeTransform "0.000000,0.000000,5000.000000") "Undefined" "MultiplyWithRoot" 0 0))
  (Transformation|AttachComponentToComponent (Variables|/Script/Engine.Actor|GetRootComponent _returnvalue) (Variables|/Game/FirstPerson/Blueprints/BP_FirstPersonCharacter.BP_FirstPersonCharacter_C|GetFirstPersonMesh (Variables|Default|GetCharacter)) "hand" "SnapToTarget" "SnapToTarget" "SnapToTarget" true))

(event Collision|EventActorBeginOverlap
  (params (OtherActor :type Actor%20Object%20Reference)))

(event EventTick
  (params (DeltaSeconds :type Float%20%28single-precision%29)))

(fn ConstructionScript
  (|CallParentFunction))