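; BP_EnemyBase is an enemy character that chases the player and deals damage on contact.
; Tick reissues AIMoveTo toward player 0 unless the airborne flag is set.
; Taking damage updates the health widget and switches movement to Falling for a second, pausing the chase, before destroying the enemy if health is depleted.
; Sphere overlap with the first-person character applies damage through its BP_MyController.
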(event OnComponentBeginOverlap(Sphere)
  (params (OverlappedComponent :type Primitive%20Component%20Object%20Reference) (OtherActor :type Actor%20Object%20Reference) (OtherComp :type Primitive%20Component%20Object%20Reference) (OtherBodyIndex :type Integer) (bFromSweep :type Boolean) (SweepResult :type Hit%20Result%20Structure%20%28by%20ref%29))
  (bind _asbp_first_person_character (Utilities|Casting|CastToBP_FirstPersonCharacter OtherActor))
  (bind _asbp_my_controller (Utilities|Casting|CastToBP_MyController (Pawn|GetController _asbp_first_person_character)))
  (Default|ApplyDamage _asbp_my_controller (Variables|Default|GetDamageAmount)))

(event EventBeginPlay
  (bind _aswbp_enemy_health (Utilities|Casting|CastToWBP_EnemyHealth (UserInterface|GetUserWidgetObject (Variables|Default|GetWidget_0))))
  (bind _output_get (Variables|Default|SetWBP%20Enemy%20Health _aswbp_enemy_health))
  (Variables|/Game/Health/UI/WBP_EnemyHealth.WBP_EnemyHealth_C|SetCurrentHealth _output_get (Variables|Default|GetCurrentHealth))
  (Variables|/Game/Health/UI/WBP_EnemyHealth.WBP_EnemyHealth_C|SetMaxHealth _output_get (Variables|Default|GetMaxHealth)))

(event EventTick
  (params (DeltaSeconds :type Float%20%28single-precision%29))
  (if (not (Variables|Default|GetIsInAir?))
    (AI|AIMoveTo self (Transformation|GetWorldLocation (Variables|/Script/Engine.Character|GetCapsuleComponent (Game|GetPlayerCharacter 0))) 0 5e+01 true)))

(event Game|Damage|EventAnyDamage
  (params (Damage :type Float%20%28single-precision%29) (DamageType :type Damage%20Type%20Object%20Reference) (InstigatedBy :type Controller%20Object%20Reference) (DamageCauser :type Actor%20Object%20Reference))
  (bind _output_get (Variables|Default|SetCurrentHealth (- (Variables|Default|GetCurrentHealth) Damage)))
  (Default|UpdateHealth (Variables|Default|GetWBP%20Enemy%20Health) _output_get)
  (Variables|Default|SetIsInAir? true)
  (Pawn|Components|CharacterMovement|SetMovementMode (Variables|Character|GetCharacterMovement) "MOVE_Falling" 0)
  (Utilities|FlowControl|Delay 1.0)
  (Pawn|Components|CharacterMovement|SetMovementMode (Variables|Character|GetCharacterMovement) "MOVE_Walking" 0)
  (Variables|Default|SetIsInAir? false)
  (if (<= (Variables|Default|GetCurrentHealth) 0)
    (Actor|DestroyActor)))

(fn ConstructionScript)